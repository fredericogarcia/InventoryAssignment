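; Inventory component that stores items as ID and quantity pairs in a slot array, sized on BeginPlay.
; AddToInventory reads DataTable_Item, then adds stackable items to a stack below max size or fills an empty slot.
; It adds the whole quantity without clamping or splitting, and prints errors for invalid items or no free slot.
; RemoveFromInventory is an empty stub, and Map-based add nodes are left unconnected.
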(event EventBeginPlay
  ;[1 1 1] Sets the maximum size of the array
  (Utilities|Array|Resize (Variables|Default|GetInventory) (Variables|Default|GetInventorySIze)))

(fn AddtoInventory
  (params (ItemID :type Name%20%28by%20ref%29) (Quantity :type Integer))
  (bind (_success _slotindex) (CallFunction|FindEmptySlot))
  (bind (_success_2 _slotindex_2) (CallFunction|FindEmptySlot))
  (bind _inventory (Variables|Default|GetInventory))
  (bind _item_index (CallFunction|FindItemSlotandCheckforSpace ItemID))
  (bind _output (Utilities|Array|Get(acopy) _inventory _item_index))
  ;[1 1 1] Checks if item is stackable
  (bind _returnvalue (Utilities|GetDataTableRow "/Game/Inventory/DataTable_Item.DataTable_Item" ItemID)
    (:then
      (if (Utilities|Struct|BreakStruct_Item _returnvalue)
        ;[1 1 1] Finds the correct item, in the correct slot, and checks for space
        (if (.SlotWithSpace (CallFunction|FindItemSlotandCheckforSpace ItemID))
          ;[1 1 1] Adds to existing stack
          (Utilities|Array|SetArrayElem (Variables|Default|GetInventory) _item_index (Utilities|Struct|MakeStruct_Slot (.itemid _output) (+ Quantity (.quantity _output))))
          (return true)
          (else
            ;[1 1 1] Creates a new stack, if inventory full return error
            (if _success_2
              (Utilities|Array|SetArrayElem (Variables|Default|GetInventory) _slotindex_2 (Utilities|Struct|MakeStruct_Slot ItemID Quantity))
              (return true)
              (else
                (Development|PrintString "Inventory Full")
                (return false)))))
        (else
          ;[1 1 1] If FindEmptySlot is true, Adds non stackable items to inventory, else returns error
          (if _success
            (Utilities|Array|SetArrayElem (Variables|Default|GetInventory) _slotindex (Utilities|Struct|MakeStruct_Slot ItemID Quantity))
            (return true)
            (else
              (Development|PrintString "Inventory Full")
              (return false))))))
    (:RowNotFound
      ;[1 1 1] Item doesnt exist in data table
      (Development|PrintString "Invalid Item")
      (return false))))

(fn RemovefromInventory)

(fn FindItem
  (params (ItemID :type Name))
  (for (_array_element _array_index) (Variables|Default|GetInventory)
    (if (== (.ItemID (Utilities|Struct|BreakStruct_Slot _array_element)) ItemID)
      (return _array_index (.Quantity (Utilities|Struct|BreakStruct_Slot _array_element)))))
  (return -1 -1))

(fn FindEmptySlot
  (for (_array_element _array_index) (Variables|Default|GetInventory)
    (if (== (.Quantity (Utilities|Struct|BreakStruct_Slot _array_element)) 0)
      (return true _array_index)))
  (return false -1))

(fn FindItemMaxStackSize
  (params (ItemID :type Name))
  (bind _returnvalue (Utilities|GetDataTableRow "/Game/Inventory/DataTable_Item.DataTable_Item" ItemID)
    (:then
      (return (.stacksize _returnvalue)))
    (:RowNotFound
      (return -1))))

(fn FindItemSlotandCheckforSpace
  (params (ItemID :type Name))
  (for (_array_element _array_index) (Variables|Default|GetInventory)
    (if (== (.itemid _array_element) ItemID)
      (if (< (.quantity _array_element) (CallFunction|FindItemMaxStackSize ItemID))
        (return true _array_index))))
  (return false -1))