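; BP_Item is a world pickup that adds its ItemID and Quantity to an overlapping third-person character's inventory component, then destroys itself after a brief delay.
; The construction script looks up ItemID in the item data table to set the name and static mesh.
; A widget component shows quantity and name, and turns every tick to face the player camera.
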(event EventBeginPlay
  ;[1 1 1] Displays world space quantity and item name
  (bind _asw_pickup_item (Utilities|Casting|CastToW_PickupItem (UserInterface|GetWidget (Variables|Default|GetWidget))))
  (Variables|/Game/Inventory/Widgets/W_PickupItem.W_PickupItem_C|SetItemTextName _asw_pickup_item (Utilities|String|Append (Utilities|String|ToString(Integer) (Variables|Default|GetQuantity)) "x" " " (Variables|Default|GetName))))

(event EventTick
  (params (DeltaSeconds :type Float%20%28single-precision%29))
  ;[1 1 1] updates the text rotation to always face the players camera
  (Transformation|SetWorldRotation (Variables|Default|GetWidget) (Math|Rotator|FindLookatRotation (Transformation|GetWorldLocation (Variables|Default|GetWidget)) (Transformation|GetWorldLocation (Variables|/Script/Engine.PlayerCameraManager|GetTransformComponent (Game|GetPlayerCameraManager 0)))) false false))

(event Collision|EventActorBeginOverlap
  (params (OtherActor :type Actor%20Object%20Reference))
  ;[1 1 1] Adds item to inventory, and destroy actor
  (bind _asbp_third_person_character (Utilities|Casting|CastToBP_ThirdPersonCharacter OtherActor))
  (Utilities|IsValid (Variables|/Game/Inventory/BP_ThirdPersonCharacter.BP_ThirdPersonCharacter_C|GetBPC_Inventory _asbp_third_person_character)
    (:Is%20Valid
      (Default|AddtoInventory (Variables|/Game/Inventory/BP_ThirdPersonCharacter.BP_ThirdPersonCharacter_C|GetBPC_Inventory _asbp_third_person_character) (Variables|Default|GetItemID) (Variables|Default|GetQuantity))
      (if true
        (Utilities|FlowControl|Delay 0.01)
        (Actor|DestroyActor)))))

(fn ConstructionScript
  ;[1 1 1] Gets info from data table to know which mesh needs to be set
  (bind _returnvalue (Utilities|GetDataTableRow "/Game/Inventory/DataTable_Item.DataTable_Item" (Variables|Default|GetItemID))
    (:then
      (Variables|Default|SetName (.Name (Utilities|Struct|BreakStruct_Item _returnvalue)))
      (Components|StaticMesh|SetStaticMesh (Variables|Default|GetStaticMesh) (.StaticMesh (Utilities|Struct|BreakStruct_Item _returnvalue))))))