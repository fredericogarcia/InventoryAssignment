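; Player controller that opens the inventory and crafting screen when the Inventory input action is pressed.
; It shows the mouse cursor only if a keyboard key triggered the action, hiding it for other inputs.
; Each press creates and stores a new W_InventoryAndCrafting widget, adds it to the viewport and switches to UI-only input focused on it.
; The controller contains no logic for closing the screen or restoring game input.
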(event Input|ActionEvents|InputActionInventory
  (params (Key :type Key%20Structure :default "None"))
  (bind _self self)
  (:Pressed
    (if (Class|KismetInputLibrary|KeyIsKeyboardKey Key)
      (Variables|/Script/Engine.PlayerController|SetbShowMouseCursor _self true)
      (else
        (Variables|/Script/Engine.PlayerController|SetbShowMouseCursor _self false)))
    (bind _returnvalue (UserInterface|CreateWidget "/Game/Inventory/Widgets/W_InventoryAndCrafting.W_InventoryAndCrafting_C"))
    (bind _output_get (Variables|Default|SetInventoryWidget _returnvalue))
    (UserInterface|Viewport|AddtoViewport _output_get 0)
    (Input|SetInputModeUIOnly self (Variables|Default|GetInventoryWidget) "LockOnCapture" false)))

(fn ConstructionScript)